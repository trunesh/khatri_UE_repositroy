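; Plunger actor, apparently for launching a ball, with a pull-back and release motion.
; ChargePlunger plays a timeline that lerps the Plunger component along its local Y axis from its rest position.
; Stopplunger halts that timeline and uses MoveComponentTo to return the component over PlungerSpeed seconds.
; GetBallLocation converts the BallLocation offset from actor space to world space.
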(event `self.ReceiveBeginPlay`)

(event `ChargePlunger`
  (bind (_direction _newtrack_0) (`Timeline|ChargePlunge` :!via `PlayFromStart` :!label _label)
    (:`Update`
      (`SceneComponent.K2_SetRelativeLocation` (`self.Plunger`) (`KismetMathLibrary.VLerp` (0.0 0.0 0.0) (0.0 70.0 0.0) _newtrack_0) false false))))

(event `Stopplunger`
  (`|ExecutionSequence`
    (:`then_0`
      (goto _label :!via `Stop`))
    (:`then_1`
      (`KismetSystemLibrary.MoveComponentTo` (`self.Plunger`) (0.0 0.0 0.0) (struct) false false (`self.PlungerSpeed`)))))

(fn `Get ball location`
  (returns (BallSpawnVector :type "Vector Structure"))
  (return (`KismetMathLibrary.TransformLocation` (`self.GetTransform`) (`self.BallLocation`))))

(fn `UserConstructionScript`)