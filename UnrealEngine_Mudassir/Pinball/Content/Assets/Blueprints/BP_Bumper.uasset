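; BP_Bumper is a pinball bumper that kicks the ball away and awards points.
; On overlap with BP_Ball, it applies a velocity-change impulse along the bumper-to-ball direction, adds score through PinballGameMode and prints the result.
; A timeline then moves the bumper mechanism vertically and drives the emissive boost on a dynamic material instance created in the construction script.
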(event `self.ReceiveActorBeginOverlap`
  (params (OtherActor :type "Actor Object Reference"))
  (bind _asbp_ball (cast `/Game/Assets/Blueprints/BP_Ball` OtherActor))
  (`PrimitiveComponent.AddImpulse` (`/Game/Assets/Blueprints/BP_Ball.Ball` _asbp_ball) (* (`KismetMathLibrary.GetDirectionUnitVector` (`self.K2_GetActorLocation`) (`self.K2_GetActorLocation` _asbp_ball)) 3000.0) "None" true)
  (bind _aspinball_game_mode (cast `/Game/Assets/Blueprints/PinballGameMode` (`GameplayStatics.GetGameMode`)))
  (bind _score (`/Game/Assets/Blueprints/PinballGameMode.AddScore` _aspinball_game_mode 10.0))
  (`KismetSystemLibrary.PrintString` (`KismetStringLibrary.Conv_DoubleToString` _score))
  (bind (_direction _bumplerp) (`Timeline|Bumplerp` :!via `PlayFromStart`)
    (:`Update`
      (`SceneComponent.K2_SetRelativeLocation` (`self.BumperMechanism`) (`KismetMathLibrary.VLerp` (0.0 0.0 10.0) (0.0 0.0 -70.0) _bumplerp) false false)
      (`MaterialInstanceDynamic.SetScalarParameterValue` (`self.BumperMID`) "EmmisiveBoost" (`KismetMathLibrary.Lerp` 0.0 20.0 _bumplerp)))))

(fn `UserConstructionScript`
  (bind _returnvalue (`PrimitiveComponent.CreateDynamicMaterialInstance` (`self.bumper`) 1 null "None"))
  (set `self.BumperMID` _returnvalue))