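; Pinball player controller that maps flipper and plunger input to the table's actors.
; On BeginPlay it sorts all BP_Flipper actors into left and right arrays by FlipType and caches the first BP_Plunger.
; Plunger input charges on press and stops on release.
; Flipper input calls Flip and Flop on elements of per-side ForEach loops, but those loops are never executed.
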(event Custom|DetectFlippers
  (bind _outactors (Actor|GetAllActorsOfClass "/Game/Assets/Blueprints/BP_Flipper.BP_Flipper_C"))
  (for _array_element _outactors
    (switch Utilities|FlowControl|Switch|SwitchonFlipType (Variables|/Game/Assets/Blueprints/BP_Flipper.BP_Flipper_C|GetFlipType _array_element)
      (:NewEnumerator0
        (Utilities|Array|Add (Variables|Default|GetLeftFlippers) _array_element))
      (:NewEnumerator1
        (Utilities|Array|Add (Variables|Default|GetRightFlippers) _array_element)))))

(event Custom|DetectPlunger
  (bind _outactors (Actor|GetAllActorsOfClass "/Game/Assets/Blueprints/BP_Plunger.BP_Plunger_C"))
  (Variables|Default|SetPlunger (Utilities|Array|Get(acopy) _outactors)))

(event EventBeginPlay
  (CallFunction|DetectFlippers)
  (CallFunction|DetectPlunger))

(event EventTick
  (params (DeltaSeconds :type Float%20%28single-precision%29)))

(event Input|ActionEvents|InputActionPlungerPush
  (params (Key :type Key%20Structure :default "None"))
  (bind _plunger (Variables|Default|GetPlunger))
  (:Pressed
    (Default|ChargePlunger _plunger))
  (:Released
    (Default|Stopplunger _plunger)))

(event Input|ActionEvents|InputActionLeftFlip
  (params (Key :type Key%20Structure :default "None"))
  (:Pressed
    (Default|Flip (stale _array_element)))
  (:Released
    (Default|Flop (stale _array_element))))

(event Input|ActionEvents|InputActionRightFlip
  (params (Key :type Key%20Structure :default "None"))
  (:Pressed
    (Default|Flip (stale _array_element)))
  (:Released
    (Default|Flop (stale _array_element))))

(fn ConstructionScript)