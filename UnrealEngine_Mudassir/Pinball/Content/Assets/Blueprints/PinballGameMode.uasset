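; Pinball game mode that handles ball spawning, the game-over check and scoring.
; On BeginPlay it spawns a BP_Ball at the ball location of the first BP_Plunger found and binds to the ball's OnDestroyed.
; Each destroyed ball increments a counter and triggers a respawn until the limit of three, when it only prints "Gameover".
; AddScore adds points scaled by Multiplier to Score and returns the total.
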(event `self.ReceiveBeginPlay`
  (`self.Spawn`))

(event `Spawn`
  (bind _outactors (`GameplayStatics.GetAllActorsOfClass` "/Game/Assets/Blueprints/BP_Plunger.BP_Plunger_C"))
  (bind _ballspawnvector (`/Game/Assets/Blueprints/BP_Plunger.Get ball location` (`|GetArrayItem` _outactors)))
  (bind _returnvalue (`|SpawnActorFromClass` "/Game/Assets/Blueprints/BP_Ball.BP_Ball_C" (`KismetMathLibrary.MakeTransform` _ballspawnvector) "Undefined" "OverrideRootScale" null null))
  (add `self.OnDestroyed` _returnvalue (delegate `OnDestroy`)))

(event `OnDestroy` :!signature `self.OnDestroyed`
  (params (DestroyedActor :type "Actor Object Reference"))
  (bind _result (`/Engine/EditorBlueprintResources/StandardMacros.IncrementInt` (`self.MyCount`))
    (:`  `
      (if (< _result 3)
        (`self.Spawn`)
        (else
          (`KismetSystemLibrary.PrintString` "Gameover"))))))

(fn `AddScore`
  (params (NumberOfPoints :type "Float (double-precision)"))
  (returns (Score :type "Float (double-precision)"))
  (bind _output_get (set `self.Score` (+ (* NumberOfPoints (`self.Multiplier`)) (`self.Score`))))
  (return _output_get))

(fn `UserConstructionScript`)